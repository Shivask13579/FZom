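; BP_Zombie is an AI zombie enemy that spots the player and attacks in melee.
; Pawn sensing sets the SeeingPlayer blackboard key and starts chase music, while a looping timer clears the key and fades the music if sight stays lost.
; AttackPlayer halts movement, plays a montage and sphere-traces for damage; OnAttack's box-overlap damage is disconnected.
; TrapDoll ragdolls and destroys the zombie, but only if ZombieDead is already true.
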(event `self.ReceiveBeginPlay`
  ;[1 1 1] Event Begin Play
  (`KismetSystemLibrary.K2_SetTimerDelegate` (delegate `Stop Seeing Player`) 0.8 true))

(event `Stop Seeing Player`
  ;[1 1 1] Event Begin Play
  (`BlackboardComponent.SetValueAsBool` (`AIBlueprintHelperLibrary.GetBlackboard` (`AIBlueprintHelperLibrary.GetAIController` self)) "SeeingPlayer" false)
  (`KismetSystemLibrary.Delay` 1.0)
  (if (not (`BlackboardComponent.GetValueAsBool` (`AIBlueprintHelperLibrary.GetBlackboard` (`AIBlueprintHelperLibrary.GetAIController` self)) "SeeingPlayer"))
    (bind _chaseaudio (`self.ChaseAudio`)
      (:`then`
        (`AudioComponent.FadeOut` _chaseaudio 3.0 0.0 "Linear"))
      (:`else`))))

(event `self.PawnSensing.OnSeePawn`
  (params (Pawn :type "Pawn Object Reference"))
  ;[1 1 1] ZombieSensing
  (if (`self.ActorHasTag` Pawn "Player")
    (`BlackboardComponent.SetValueAsBool` (`AIBlueprintHelperLibrary.GetBlackboard` (`AIBlueprintHelperLibrary.GetAIController` self)) "SeeingPlayer" true)
    (`self.ChaseAudio`
      (:`then`)
      (:`else`
        (bind _returnvalue (`GameplayStatics.SpawnSound2D` "/Game/Audio/Chase.Chase" 1.0 1.0 0.0 null))
        (bind _output_get (set `self.ChaseAudio` _returnvalue))
        (`AudioComponent.FadeIn` _output_get 2.0 1.0 0.0 "Linear")))))

(event `TrapDoll`
  ;[1 1 1] Trap
  (if (`self.ZombieDead`)
    (set `self.ZombieDead` true)
    (`PrimitiveComponent.SetSimulatePhysics` (`self.Mesh`) true)
    (`KismetSystemLibrary.Delay` 1.0)
    (`self.K2_DestroyActor`)
    (`self.DisableInput` null)))

(event `Attack Player`
  (bind _attack_trace_point (`self.Attack Trace Point`))
  (bind _returnvalue (`SceneComponent.K2_GetComponentLocation` _attack_trace_point))
  ;[1 1 1] ZombieAttack
  (if (not (`self.Attacking?`))
    (set `self.Attacking?` true)
    (cast `AIController` (`self.GetController`))
    (`MovementComponent.StopMovementImmediately` (`self.CharacterMovement`))
    (`CharacterMovementComponent.SetMovementMode` (`self.CharacterMovement`) "MOVE_None" 0)
    (`|PlayMontage` (`self.Mesh`) "/Game/Enemy_AI/zombie_attack1_Montage.zombie_attack1_Montage"
      (:`then`
        (bind (_outhit _returnvalue_2) (`KismetSystemLibrary.SphereTraceSingleForObjects` :`Start` _returnvalue :`End` (+ _returnvalue (* (`KismetMathLibrary.GetForwardVector` (`SceneComponent.K2_GetComponentRotation` _attack_trace_point)) (0.0 0.0 0.0))) :`ObjectTypes` (`|MakeArray` "ObjectTypeQuery3" :!type "EObjectTypeQuery Enum") :`DrawDebugType` "ForDuration"))
        (if _returnvalue_2
          (`GameplayStatics.ApplyDamage` (`.HitActor` (`GameplayStatics.BreakHitResult` _outhit)) 15.0)
          (`CharacterMovementComponent.SetMovementMode` (`self.CharacterMovement`) "MOVE_Walking" 0 :!label _label)))
      (:`OnCompleted`
        (set `self.Attacking?` false)
        (goto _label)))))

(event `OnAttack`
  ;[1 1 1] OnAttack
  (`|PlayMontage` (`self.Mesh`) "/Game/Enemy_AI/zombie_attack1_Montage.zombie_attack1_Montage"
    (:`then`
      (bind _outactors (`KismetSystemLibrary.BoxOverlapActors` (`SceneComponent.K2_GetComponentLocation` (`self.BP_Damage`)) (`self.Attack Box Extent`) (`|MakeArray` "ObjectTypeQuery3" :!type "EObjectTypeQuery Enum") "/Game/ThirdPerson/Blueprints/MainCharacter.MainCharacter_C" (`|MakeArray` self :!type "Actor Object Reference"))))))

(fn `UserConstructionScript`)