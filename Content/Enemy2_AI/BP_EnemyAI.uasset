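; Enemy AI pawn that detects the player, plays chase music and performs a melee attack.
; PawnSensing sets the SeeingPlayer blackboard key and fades in chase audio, while a looping timer clears the key and fades audio out unless the player is re-sighted.
; Attack halts movement, plays a montage and immediately sphere-traces for damage, restoring walking on hit or montage completion.
; A Ragdoll event enables mesh physics.
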(event `self.ReceiveBeginPlay`
  ;[1 1 1] EventBeginPlay
  (`KismetSystemLibrary.K2_SetTimerDelegate` (delegate `Stop Seeing Player`) 0.8 true))

(event `Stop Seeing Player`
  ;[1 1 1] EventBeginPlay
  (`BlackboardComponent.SetValueAsBool` (`AIBlueprintHelperLibrary.GetBlackboard` (`AIBlueprintHelperLibrary.GetAIController` self)) "SeeingPlayer" false)
  (`KismetSystemLibrary.Delay` 1.0)
  (if (not (`BlackboardComponent.GetValueAsBool` (`AIBlueprintHelperLibrary.GetBlackboard` (`AIBlueprintHelperLibrary.GetAIController` self)) "SeeingPlayer"))
    (bind _chaseaudio (`self.ChaseAudio`)
      (:`then`
        (`AudioComponent.FadeOut` _chaseaudio 3.0 0.0 "Linear"))
      (:`else`))))

(event `self.PawnSensing.OnSeePawn`
  (params (Pawn :type "Pawn Object Reference"))
  ;[1 1 1] OnSensing
  (if (`self.ActorHasTag` Pawn "Player")
    (`BlackboardComponent.SetValueAsBool` (`AIBlueprintHelperLibrary.GetBlackboard` (`AIBlueprintHelperLibrary.GetAIController` self)) "SeeingPlayer" true)
    (`self.ChaseAudio`
      (:`then`)
      (:`else`
        (bind _returnvalue (`GameplayStatics.SpawnSound2D` "/Game/Audio/Chase.Chase" 1.0 1.0 0.0 null))
        (bind _output_get (set `self.ChaseAudio` _returnvalue))
        (`AudioComponent.FadeIn` _output_get 3.0 1.0 0.0 "Linear")))))

(event `Ragdoll`
  (`PrimitiveComponent.SetSimulatePhysics` (`self.Mesh`) true))

(event `Attack`
  (bind _attacktracepoint (`self.AttackTracePoint`))
  (bind _returnvalue (`SceneComponent.K2_GetComponentLocation` _attacktracepoint))
  ;[1 1 1] Attack
  (if (not (`self.Attacking`))
    (set `self.Attacking` true)
    (cast `/Game/Enemy2_AI/BP_AI_Controller` (`self.GetController`))
    (`MovementComponent.StopMovementImmediately` (`self.CharacterMovement`))
    (`CharacterMovementComponent.SetMovementMode` (`self.CharacterMovement`) "MOVE_None" 0)
    (`NavMovementComponent.StopActiveMovement` (`self.CharacterMovement`))
    (`|PlayMontage` (`self.Mesh`) "/Game/Enemy2_AI/Animations/A_Attack_Montage.A_Attack_Montage"
      (:`then`
        (bind (_outhit _returnvalue_2) (`KismetSystemLibrary.SphereTraceSingleForObjects` _returnvalue (+ _returnvalue (* (`KismetMathLibrary.GetForwardVector` (`SceneComponent.K2_GetComponentRotation` _attacktracepoint)) 50.0)) 100.0 (`|MakeArray` "ObjectTypeQuery3" :!type "EObjectTypeQuery Enum")))
        (if _returnvalue_2
          (`GameplayStatics.ApplyDamage` (`.HitActor` (`GameplayStatics.BreakHitResult` _outhit)) 30.0)
          (`CharacterMovementComponent.SetMovementMode` (`self.CharacterMovement`) "MOVE_Walking" 0 :!label _label)))
      (:`OnCompleted`
        (set `self.Attacking` false)
        (goto _label)))))

(fn `UserConstructionScript`)